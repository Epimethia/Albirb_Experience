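; Game mode that streams trees around the player by spawning new ones and culling distant ones as the pawn moves.
; Tick runs through a 0.2 second Delay, throttling a cycle that culls, then spawns one tree.
; CheckTreesInView destroys tracked trees beyond a distance threshold and removes them from TreeArray during iteration.
; SpawnTree places a query-only collision tree at a fixed height, using GeneratePoint with the pawn's position and facing, and tracks it.
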(event EventTick
  (params (DeltaSeconds :type Float%20%28single-precision%29))
  (Utilities|FlowControl|Delay 0.2)
  (CallFunction|CheckTreesinView)
  (CallFunction|SpawnTree))

(fn ConstructionScript)

(fn CheckTreesinView
  (Utilities|IsValid (Game|Player|GetPlayerPawn 0)
    (:Is%20Valid
      (for (_array_element _array_index) (Variables|Default|GetTree%20Array)
        (if (>= (Math|Vector|VectorLength (- (Transformation|GetActorLocation _array_element) (Transformation|GetActorLocation (Game|Player|GetPlayerPawn 0)))) 6.5e+03)
          (Actor|DestroyActor _array_element)
          (Utilities|Array|RemoveIndex (Variables|Default|GetTree%20Array) _array_index))))))

(fn SpawnTree
  (bind _returnvalue (Game|Player|GetPlayerPawn 0))
  (Utilities|IsValid _returnvalue
    (:Is%20Valid
      (bind _returnvalue_2 (Class|ALBIRBEXPERIENCEGameMode|GeneratePoint (Transformation|GetActorForwardVector _returnvalue) (Transformation|GetActorRotation _returnvalue) (Transformation|GetActorLocation _returnvalue)))
      (bind _returnvalue_3 (Game|SpawnActorfromClass "/Game/Maps/Environment_Assets/BP_Tree_0.BP_Tree_0_C" (Math|Transform|MakeTransform (Math|Vector|MakeVector (.x _returnvalue_2) (.y _returnvalue_2) 1e+03)) "AlwaysSpawn" 0 0))
      (Collision|SetCollisionEnabled (Variables|/Game/Maps/Environment_Assets/BP_Tree_0.BP_Tree_0_C|GetStaticMesh _returnvalue_3) "QueryOnly")
      (Utilities|Array|Add (Variables|Default|GetTree%20Array) _returnvalue_3))))