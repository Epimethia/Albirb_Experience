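; Player pawn Blueprint that opens the start menu on BeginPlay and a pause menu on the Paused input.
; StartMenu pauses the game, creates BP_MenuWidget if needed, displays it and switches to UI-only input with a visible cursor.
; PauseGame pauses and adds BP_PauseWidget only when creating it; its UI-only input step is unconnected.
; The Paused event also prints a debug string and shows the cursor.
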(event EventBeginPlay
  (CallFunction|StartMenu))

(event Collision|EventActorBeginOverlap
  (params (OtherActor :type Actor%20Object%20Reference)))

(event EventTick
  (params (DeltaSeconds :type Float%20%28single-precision%29)))

(event Input|ActionEvents|InputActionPaused
  (params (Key :type Key%20Structure))
  (:Pressed
    (Development|PrintString "Hello")
    (CallFunction|PauseGame)
    (Variables|/Script/Engine.PlayerController|SetbShowMouseCursor (Game|GetPlayerController 0) true)))

(fn ConstructionScript)

(fn StartMenu
  (bind _returnvalue (Game|GetPlayerController 0))
  ;[1 1 1] Paused the game and made sure the start menu widget exists
  (Game|SetGamePaused true)
  (Utilities|IsValid 0
    (:Is%20Valid
      _)
    (:Is%20Not%20Valid
      (bind _returnvalue_2 (UserInterface|CreateWidget "/Game/Menu/BP_MenuWidget.BP_MenuWidget_C" (Game|GetPlayerController 0)))
      (Variables|Default|SetMenuPause _returnvalue_2)))
  ;[1 1 1] Add the widget to the viewport and set the input of player to UI only and show the cursor
  (UserInterface|Viewport|AddtoViewport (Variables|Default|GetMenuPause) 0)
  (Input|SetInputModeUIOnly _returnvalue (Variables|Default|GetMenuPause) "DoNotLock")
  (Variables|/Script/Engine.PlayerController|SetbShowMouseCursor _returnvalue true))

(fn PauseGame
  ;[1 1 1] Pasues the game same process as the start menu
  (Game|SetGamePaused true)
  (Utilities|IsValid 0
    (:Is%20Not%20Valid
      (bind _returnvalue (UserInterface|CreateWidget "/Game/Menu/BP_PauseWidget.BP_PauseWidget_C" (Game|GetPlayerController 0)))
      (Variables|Default|SetPause _returnvalue)
      (UserInterface|Viewport|AddtoViewport (Variables|Default|GetPause) 0))))