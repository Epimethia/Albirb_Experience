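; Game mode Blueprint that holds the pause menu logic and enables player character input on BeginPlay.
; MainMenu pauses the game, creates BP_MenuWidget if none is cached in Pause, shows it and switches to UI-only input with a cursor.
; SwitchToGameScreen unpauses, removes all widgets and restores game-only input.
; The Pause input release only prints a debug string; the MainMenu call in the event graph is unwired.
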(event EventBeginPlay
  (Input|EnableInput (Game|GetPlayerCharacter 0) (Game|GetPlayerController 0)))

(event EventTick
  (params (DeltaSeconds :type Float%20%28single-precision%29)))

(event Input|ActionEvents|InputActionPause
  (params (Key :type Key%20Structure))
  (:Released
    (Development|PrintString "Hello")))

(fn ConstructionScript)

(fn MainMenu
  ;[1 1 1] Pauses the game, see if there is a menu widget created, create widget if not exist and add pause variable
  (Game|SetGamePaused true)
  (Utilities|IsValid 0
    (:Is%20Valid
      _)
    (:Is%20Not%20Valid
      (bind _returnvalue (UserInterface|CreateWidget "/Game/Menu/BP_MenuWidget.BP_MenuWidget_C"))
      (Variables|Default|SetPause _returnvalue)))
  ;[1 1 1] Add widget to viewport and set the input only for UI and show the cursor
  (UserInterface|Viewport|AddtoViewport (Variables|Default|GetPause) 0)
  (Input|SetInputModeUIOnly (Game|GetPlayerController 0) (Variables|Default|GetPause) "DoNotLock")
  (Variables|/Script/Engine.PlayerController|SetbShowMouseCursor (Game|GetPlayerController 0) true))

(fn SwitchtoGameScreen
  (bind _returnvalue (Game|GetPlayerController 0))
  ;[1 1 1] Unpause game, delete the menu widget, make input only towards game and disable cursor
  (Game|SetGamePaused false)
  (Viewport|RemoveAllWidgets)
  (Input|SetInputModeGameOnly _returnvalue)
  (Variables|/Script/Engine.PlayerController|SetbShowMouseCursor _returnvalue false))